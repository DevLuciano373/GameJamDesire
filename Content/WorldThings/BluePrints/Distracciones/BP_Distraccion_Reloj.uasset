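; BP_Distraccion_Reloj is a clock distraction pickup that rotates continuously, lures overlapping characters toward its spawn position and drains their spirituality.
; Entering RangoDistraccion sends the attraction and spirituality-loss messages, while any actor end overlap sends messages ending attraction and spirituality changes.
; Entering the RangoDesaparecer range sends a touch message with five times the spiritual damage, then destroys the actor.
; All effects are delegated to the other actor through interface messages.
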(event `self.ReceiveBeginPlay`
  (set `self.PosicionDistraccion` (`self.K2_GetActorLocation`)))

(event `self.ReceiveTick`
  (params (DeltaSeconds :type "Float (single-precision)"))
  (`self.K2_AddActorLocalRotation` (struct :`Pitch` 1.0 :`Yaw` 1.0 :`Roll` 1.0)))

(event `self.RangoDistraccion.OnComponentBeginOverlap`
  (params (OverlappedComponent :type "PrimitiveComponent Object Reference") (OtherActor :type "Actor Object Reference") (OtherComp :type "PrimitiveComponent Object Reference") (OtherBodyIndex :type Integer) (bFromSweep :type Boolean) (SweepResult :type "HitResult Structure (by ref)"))
  (`|ExecutionSequence`
    (:`then_0`
      (message `/Game/WorldThings/Interfaces/BPI_Distraer.AtraerPersonaje` OtherActor (`self.PosicionDistraccion`)))
    (:`then_1`
      (message `/Game/WorldThings/Interfaces/BPI_Espiritualidad.PerderEspiritualidad` OtherActor (`self.DañoEspiritual`)))))

(event `self.ReceiveActorEndOverlap`
  (params (OtherActor :type "Actor Object Reference"))
  (`|ExecutionSequence`
    (:`then_0`
      (message `/Game/WorldThings/Interfaces/BPI_Distraer.FinalizarAtraccionPersonaje` OtherActor))
    (:`then_1`
      (message `/Game/WorldThings/Interfaces/BPI_Espiritualidad.FinalizarAumentoEspiritualidad` OtherActor))
    (:`then_2`
      (message `/Game/WorldThings/Interfaces/BPI_Espiritualidad.FinalizarDañoEspirtualidad` OtherActor))))

(event `self.RangoDesaparecer.OnComponentBeginOverlap`
  (params (OverlappedComponent :type "PrimitiveComponent Object Reference") (OtherActor :type "Actor Object Reference") (OtherComp :type "PrimitiveComponent Object Reference") (OtherBodyIndex :type Integer) (bFromSweep :type Boolean) (SweepResult :type "HitResult Structure (by ref)"))
  (message `/Game/WorldThings/Interfaces/BPI_Espiritualidad.TocarDistraccion` OtherActor (* (`self.DañoEspiritual`) 5))
  (`self.K2_DestroyActor`))

(fn `UserConstructionScript`)